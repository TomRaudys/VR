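; BP_Radio is a radio with a physical button that a BP_MotionController presses by overlapping its box to toggle a classical radio stream.
; Each press plays a timeline that lowers the button mesh, then a FlipFlop drives RadioToggle to either open the media URL or pause playback.
; A DoOnce reset after a short delay debounces repeated presses.
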(event OnComponentBeginOverlap(Box)
  (params (OverlappedComponent :type Primitive%20Component%20Object%20Reference) (OtherActor :type Actor%20Object%20Reference) (OtherComp :type Primitive%20Component%20Object%20Reference) (OtherBodyIndex :type Integer) (bFromSweep :type Boolean) (SweepResult :type Hit%20Result%20Structure%20%28by%20ref%29))
  (Utilities|Casting|CastToBP_MotionController OtherActor)
  (CallFunction|ButtonPress))

(event Custom|ButtonPress
  (bind _sm_button (Variables|Default|GetSM_Button))
  (bind _relativelocation (Variables|/Script/Engine.SceneComponent|GetRelativeLocation _sm_button))
  (Utilities|FlowControl|Sequence
    (:then_0
      (Utilities|FlowControl|DoOnce false :!label _label
        (:Completed
          (bind _alpha (Timeline|MoveButton PlayFromStart)
            (:Update
              (Transformation|SetRelativeLocation _sm_button (Math|Vector|MakeVector (.x _relativelocation) (.y _relativelocation) (Math|Float|Lerp 1e+01 8.0 _alpha)) false false))
            (:Finished
              (bind _isa (Utilities|FlowControl|FlipFlop)
                (:A
                  _)
                (:B
                  _))
              (CallFunction|RadioToggle _isa))))))
    (:then_1
      (Utilities|FlowControl|Delay 1.1)
      (goto _label Reset))))

(fn ConstructionScript)

(fn RadioToggle
  (params (On? :type Boolean))
  (bind _media (Variables|Default|GetMedia))
  (if On?
    (Class|MediaPlayer|OpenUrl _media (Variables|Default|GetClassicalRadio))
    (else
      (Sequencer|Player|Pause _media))))
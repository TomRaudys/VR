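; BP_TeleportTerrain is a box-defined area that lays a grid of square tile meshes over the ground, apparently as a teleport surface.
; CreateGrid steps across the box bounds by GridSize and runs a vertical Visibility trace at each point.
; Hits spawn scaled mesh components snapped to the grid in XY, raised slightly above the impact.
; The grid builds on BeginPlay, or in construction when Finalise is set; ActiveCheck exposes the Active flag.
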(event EventBeginPlay
  (CallFunction|CreateGrid))

(event Collision|EventActorBeginOverlap
  (params (OtherActor :type Actor%20Object%20Reference)))

(event EventTick
  (params (DeltaSeconds :type Float%20%28single-precision%29)))

(fn ConstructionScript
  (bind _box (Variables|Default|GetBox))
  (bind _boxsize (Variables|Default|GetBoxSize))
  (Transformation|SetWorldScale3D _box "1.000000,1.000000,1.000000")
  (Components|Box|SetBoxExtent _box (Math|Vector|MakeVector (.x _boxsize) (.y _boxsize) 2.0) true)
  (Transformation|SetActorRotation "0, 0, 0")
  (if (Variables|Default|GetFinalise?)
    (CallFunction|CreateGrid)))

(fn CreateGrid
  (bind _box (Variables|Default|GetBox))
  (bind _box_2 (Variables|Default|GetBox))
  (bind (_origin _boxextent) (Collision|GetComponentBounds _box))
  (bind (_origin_2 _boxextent_2) (Collision|GetComponentBounds _box_2))
  (bind (_x _y) (Math|Vector|BreakVector _boxextent_2))
  (bind (_x_2 _y_2) (Math|Vector|BreakVector _origin_2))
  (LocalVariables|SetXTimes (Math|Float|Truncate (/ (Math|Float|Absolute(Float) (- (+ _x_2 _x) (- _x_2 _x))) (Variables|Default|GetGridSize))))
  (LocalVariables|SetYTimes (Math|Float|Truncate (/ (Math|Float|Absolute(Float) (- (+ _y_2 _y) (- _y_2 _y))) (Variables|Default|GetGridSize))))
  ;[1 1 1] Spawn a tile at each point
  (for _index (range 0 (LocalVariables|GetXTimes))
    (for _index_2 (range 0 (LocalVariables|GetYTimes))
      (CallFunction|TraceandSpawnSquares (Math|Vector|MakeVector (+ (* _index (Variables|Default|GetGridSize)) (- (.x _origin) (.x _boxextent))) (+ (* _index_2 (Variables|Default|GetGridSize)) (- (.y _origin) (.y _boxextent))) (.z _origin))))))

(fn TraceandSpawnSquares
  (params (Location :type Vector))
  (bind _gridsize (Variables|Default|GetGridSize))
  (bind _returnvalue (/ _gridsize 1e+02))
  (bind _returnvalue_2 (Math|Float|MakeLiteralFloat _returnvalue))
  (bind (_outhit _returnvalue_3) (Collision|LineTraceByChannel (+ Location (Math|Vector|MakeVector 0.0 0.0 (Variables|Spawn|GetTopHeight))) (- Location (Math|Vector|MakeVector 0.0 0.0 (Variables|Spawn|GetBottomHeight))) "TraceTypeQuery1" true 0 "None"))
  (if _returnvalue_3
    (bind _returnvalue_4 (AddComponent|AddStaticMeshComponent false (Math|Transform|MakeTransform (Math|Transform|InverseTransformLocation (Transformation|GetActorTransform) (Math|Vector|MakeVector (.x (Class|KismetMathLibrary|VectorSnappedtoGrid (.ImpactPoint (Collision|BreakHitResult _outhit)) (Variables|Default|GetGridSize))) (.y (Class|KismetMathLibrary|VectorSnappedtoGrid (.ImpactPoint (Collision|BreakHitResult _outhit)) (Variables|Default|GetGridSize))) (+ (.Z (Math|Vector|BreakVector (.ImpactPoint (Collision|BreakHitResult _outhit)))) (Variables|Spawn|GetSquareHeightFromGround)))) "0, 0, 0" "1,1,1")))
    (Transformation|SetWorldScale3D _returnvalue_4 (Math|Vector|MakeVector _returnvalue_2 _returnvalue_2 _returnvalue_2))))

(fn ActiveCheck
  (return (Variables|Default|GetActive)))
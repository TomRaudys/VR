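; Blueprint function library for VR-style hand grabbing that attaches actors to a hand mesh through BP_GrabPoint child actors.
; AttachToHand activates the grab point's hand visual, snaps the actor to the hand, then rotates and offsets it so the grab point aligns with the hand.
; The right hand gets an extra 180-degree flip.
; Helpers deactivate an actor's grab points or activate one as a left hand.
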(fn AttachtoHand
  (params (Actor :type Actor%20Object%20Reference) (GrabChild :type Child%20Actor%20Component%20Object%20Reference) (GrabbingHandMesh :type Skeletal%20Mesh%20Component%20Object%20Reference) (Hand :type EControllerHand%20Enum :default "Left") (UseSameAnimation :type Boolean))
  ;[1 1 1] Set initial variables
  (LocalVariables|SetActorRefLocal Actor)
  (LocalVariables|SetGrabbingHandMeshLocal GrabbingHandMesh)
  (LocalVariables|SetGrabChildLocal GrabChild)
  (LocalVariables|SetHandLocal Hand)
  ;[1 1 1] Activate hand visual
  (bind _asbp_grab_point (Utilities|Casting|CastToBP_GrabPoint (Variables|/Script/Engine.ChildActorComponent|GetChildActor (LocalVariables|GetGrabChildLocal))))
  (Default|Activate _asbp_grab_point (LocalVariables|GetGrabbingHandMeshLocal) (LocalVariables|GetHandLocal) UseSameAnimation)
  ;[1 1 1] Attach actor to player hand
  (Transformation|AttachComponentToComponent (Variables|/Script/Engine.Actor|GetRootComponent (LocalVariables|GetActorRefLocal)) (LocalVariables|GetGrabbingHandMeshLocal) "None" "SnapToTarget" "SnapToTarget" "KeepWorld" false)
  ;[1 1 1] Make sure child hand on actor aligns with player's actual hand which is now the new pivot
  (Transformation|SetRelativeRotation (Variables|/Script/Engine.Actor|GetRootComponent (LocalVariables|GetActorRefLocal)) (Math|Rotator|CombineRotators (Variables|/Script/Engine.SceneComponent|GetRelativeRotation (LocalVariables|GetGrabChildLocal)) (select (Utilities|Enum|Equal(Enum) (LocalVariables|GetHandLocal) "Right") "0.000000,0.000000,180.000000" "0, 0, 0")) false false)
  (Transformation|AddActorWorldOffset (LocalVariables|GetActorRefLocal) (- (Transformation|GetWorldLocation (LocalVariables|GetGrabbingHandMeshLocal)) (Transformation|GetWorldLocation (LocalVariables|GetGrabChildLocal)))))

(fn DeactivateHands
  (params (Actor :type Actor%20Object%20Reference))
  (for _array_element (Actor|GetAllChildActors Actor true)
    (bind _asbp_grab_point (Utilities|Casting|CastToBP_GrabPoint _array_element))
    (Default|Deactivate _asbp_grab_point)))

(fn ActiavteHandVisual
  (params (Target :type Child%20Actor%20Component%20Object%20Reference))
  (bind _asbp_grab_point (Utilities|Casting|CastToBP_GrabPoint (Variables|/Script/Engine.ChildActorComponent|GetChildActor Target)))
  (Default|Activate _asbp_grab_point 0 "Left" false))
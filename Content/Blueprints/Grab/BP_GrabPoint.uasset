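; BP_GrabPoint is a grab point that displays a posed copy of the grabbing hand on its parent actor.
; The construction script applies the pose animation to its skeletal mesh, which stays hidden from game start.
; On Activate from the parent, it copies the hand's mesh, scale and first material, flips the rotation for left hands, then shows it.
; Deactivate hides it again on release.
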(event Custom|Activate
  (params (HandMesh :type Skeletal%20Mesh%20Component%20Object%20Reference) (Hand :type EControllerHand%20Enum :default "Left"))
  ;[1 1 1] Call activate from parent actor
  (CallFunction|UpdateHandVisual HandMesh Hand)
  (Development|SetHiddeninGame (Variables|SkeletalMeshActor|GetSkeletalMeshComponent) false true))

(event Custom|Deactivate
  ;[1 1 1] Call deactive from parent actor on let go
  (Development|SetHiddeninGame (Variables|SkeletalMeshActor|GetSkeletalMeshComponent) true true))

(event EventBeginPlay
  ;[1 1 1] Hide at start of game
  (Development|SetHiddeninGame (Variables|SkeletalMeshActor|GetSkeletalMeshComponent) true true))

(fn ConstructionScript
  (Components|Animation|OverrideAnimationData (Variables|SkeletalMeshActor|GetSkeletalMeshComponent) (Variables|Default|GetAnimation) true true 0.0 1.0))

(fn UpdateHandVisual
  (params (HandLocal :type Skeletal%20Mesh%20Component%20Object%20Reference) (Hand :type EControllerHand%20Enum :default "Left"))
  (LocalVariables|SetHandLocal2 HandLocal)
  (Transformation|SetRelativeRotation (Variables|SkeletalMeshActor|GetSkeletalMeshComponent) (select (Utilities|Enum|Equal(Enum) Hand "Left") "0.000000, 0,180.000000" "0, 0, 0") false false)
  (Class|SkinnedMeshComponent|SetSkeletalMesh (Variables|SkeletalMeshActor|GetSkeletalMeshComponent) (Variables|/Script/Engine.SkinnedMeshComponent|GetSkeletalMesh (LocalVariables|GetHandLocal2)) true)
  (Transformation|SetWorldScale3D (Variables|SkeletalMeshActor|GetSkeletalMeshComponent) (Transformation|GetWorldScale (LocalVariables|GetHandLocal2)))
  (Rendering|Material|SetMaterial (Variables|SkeletalMeshActor|GetSkeletalMeshComponent) 0 (Rendering|Material|GetMaterial (LocalVariables|GetHandLocal2) 0)))